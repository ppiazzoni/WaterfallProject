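; BP_GlobalWind is an actor that sets the global wind used by materials through the MPC_Wind parameter collection.
; WindUpdate writes the wind speed and strength variables as scalar parameters and the Arrow component's forward vector as the wind direction.
; It runs in the construction script and again on BeginPlay, with no per-frame update.
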(event EventBeginPlay
  (CallFunction|WindUpdate))

(event Collision|EventActorBeginOverlap
  (params (OtherActor :type Actor%20Object%20Reference)))

(event EventTick
  (params (DeltaSeconds :type Float%20%28single-precision%29)))

(fn ConstructionScript
  (CallFunction|WindUpdate))

(fn WindUpdate
  (Rendering|Material|SetScalarParameterValue "/Game/Waterfall_Assets/Materials/MPC_Wind.MPC_Wind" "Wind_Speed" (Variables|Default|GetWind_Speed) :!class /Script/Engine.KismetMaterialLibrary)
  (Rendering|Material|SetScalarParameterValue "/Game/Waterfall_Assets/Materials/MPC_Wind.MPC_Wind" "Wind_Strength" (Variables|Default|GetWind_Strength) :!class /Script/Engine.KismetMaterialLibrary)
  (Rendering|Material|SetVectorParameterValue "/Game/Waterfall_Assets/Materials/MPC_Wind.MPC_Wind" "Wind_Direction" (Math|Conversions|ToLinearColor(Vector) (Math|Vector|GetForwardVector (Variables|Default|GetArrow))) :!class /Script/Engine.KismetMaterialLibrary))